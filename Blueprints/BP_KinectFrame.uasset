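; Actor that displays one Kinect sensor frame type on a plane, with a text label naming that type.
; The construction script sets the label text and size.
; On BeginPlay it initializes the sensor, scales the plane to the frame's aspect ratio and offsets the label vertically to match.
; It enables the selected frame and feeds the returned texture into a dynamic material instance on the plane.
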(event EventBeginPlay
  (bind _plane (Variables|Default|GetPlane))
  (bind _frametype (Variables|KinectFrame|GetFrameType))
  (bind _returnvalue (Class|NeoKinectManager|GetFrameSize _frametype))
  (bind (_x _y) (Utilities|Struct|BreakIntPoint _returnvalue))
  (bind _returnvalue_2 (Math|Conversions|ToFloat(Integer) _y))
  (bind _returnvalue_3 (Math|Conversions|ToFloat(Integer) _x))
  (bind _returnvalue_4 (/ _returnvalue_2 _returnvalue_3))
  (Class|NeoKinectManager|InitSensor)
  (Utilities|FlowControl|Sequence
    (:then_0
      (Transformation|SetRelativeScale3D _plane (Math|Vector|MakeVector 1.0 _returnvalue_4 1.0))
      (bind _returnvalue_5 (Rendering|Material|CreateDynamicMaterialInstance _plane 0 0 :!class /Script/Engine.PrimitiveComponent))
      (bind _returnvalue_6 (Class|NeoKinectManager|SetUseFrame (Variables|KinectFrame|GetFrameType) true))
      (Rendering|Material|SetTextureParameterValue _returnvalue_5 "Texture" _returnvalue_6))
    (:then_1
      (Transformation|SetRelativeLocation (Variables|Default|GetLabel) (Math|Vector|MakeVector 0.0 0.0 (* _returnvalue_4 5e+01)) false false))))

(fn ConstructionScript
  (bind _label (Variables|Default|GetLabel))
  (Rendering|Components|TextRender|SetText _label (Utilities|Text|ToText(String) (Utilities|String|EnumtoString (Variables|KinectFrame|GetFrameType))))
  (Rendering|Components|TextRender|SetWorldSize _label (Variables|KinectFrame|GetTextSize)))