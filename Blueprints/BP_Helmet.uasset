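; BP_Helmet is a helmet mask actor that follows a tracked face and shows only while that face is tracked.
; At BeginPlay it picks a colored mask material from the Face index and creates dynamic materials for both eyes.
; While tracking, Tick copies the face's color location and orientation to the mesh's relative transform and switches off each eye's emissive glow when that eye is closed.
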(event OnFaceBeginTrack(Face)
  (params (FaceIndex :type Integer))
  (Rendering|SetActorHiddenInGame false))

(event OnFaceLost(Face)
  (params (FaceIndex :type Integer))
  (Rendering|SetActorHiddenInGame true))

(event EventBeginPlay
  (bind _staticmesh (Variables|Default|GetStaticMesh))
  (Rendering|Material|SetMaterial (Variables|Default|GetStaticMesh) 0 (Utilities|Select :Index (Variables|/Script/NeoKinectUnreal.NeoKinectFace|GetIndex (Variables|Default|GetFace)) :Option%200 "/Game/NeoKinectDemos/Materials/MI_Mask_Black.MI_Mask_Black" :Option%201 "/Game/NeoKinectDemos/Materials/MI_Mask_Red.MI_Mask_Red" :Option%202 "/Game/NeoKinectDemos/Materials/MI_Mask_Green.MI_Mask_Green" :Option%203 "/Game/NeoKinectDemos/Materials/MI_Mask_Yellow.MI_Mask_Yellow" :Option%204 "/Game/NeoKinectDemos/Materials/MI_Mask_Blue.MI_Mask_Blue" :Option%205 "/Game/NeoKinectDemos/Materials/MI_Mask_Pink.MI_Mask_Pink"))
  (bind _returnvalue (Rendering|Material|CreateDynamicMaterialInstance _staticmesh 1 0 :!class /Script/Engine.PrimitiveComponent))
  (Variables|Default|SetLeftEye _returnvalue)
  (bind _returnvalue_2 (Rendering|Material|CreateDynamicMaterialInstance _staticmesh 2 0 :!class /Script/Engine.PrimitiveComponent))
  (Variables|Default|SetRightEye _returnvalue_2)
  (Rendering|SetActorHiddenInGame true))

(event EventTick
  (params (DeltaSeconds :type Float%20%28single-precision%29))
  (bind _face (Variables|Default|GetFace))
  (bind _face_2 (Variables|Default|GetFace))
  (if (Variables|/Script/NeoKinectUnreal.NeoKinectFace|GetbIsTracked _face)
    (Utilities|FlowControl|Sequence
      (:then_0
        (Rendering|Material|SetScalarParameterValue (Variables|Default|GetLeftEye) "EmissivePower" (Utilities|Select :Index (Class|NeoKinectFace|GetEyeClosed _face "Left") :Unknown 1.0 :No 1.0 :Maybe 1.0 :Yes 0.0) :!class /Script/Engine.MaterialInstanceDynamic))
      (:then_1
        (Rendering|Material|SetScalarParameterValue (Variables|Default|GetRightEye) "EmissivePower" (Utilities|Select :Index (Class|NeoKinectFace|GetEyeClosed _face "Right") :Unknown 1.0 :No 1.0 :Maybe 1.0 :Yes 0.0) :!class /Script/Engine.MaterialInstanceDynamic))
      (:then_2
        (Transformation|SetRelativeLocationAndRotation (Variables|Default|GetStaticMesh) (Variables|/Script/NeoKinectUnreal.NeoKinectFace|GetColorLocation _face_2) (Variables|/Script/NeoKinectUnreal.NeoKinectFace|GetOrientation _face_2) false true)))))

(fn ConstructionScript)