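; Kinect face-tracking exhibit actor that shows the sensor's color feed with a helmet for each face.
; BeginPlay starts the sensor and spawns a BP_Helmet per face under Helmets.
; SetBackground streams the color frame onto a plane scaled by FOV tangent and distance to fill the camera, which matches the sensor's FOV and aspect.
; Trigger overlap shows a prompt and enables E to blend between player and Kinect views; leaving restores the player view.
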(event Custom|SetBackground
  (bind _returnvalue (Class|NeoKinectManager|GetFrameFieldOfView "Color"))
  (bind _returnvalue_2 (Class|NeoKinectManager|GetFrameSize "Color"))
  (bind _colorframe (Variables|Default|GetColorFrame))
  (bind _camera (Variables|Default|GetCamera))
  (bind (_x _y) (Utilities|Struct|BreakIntPoint _returnvalue_2))
  (bind _returnvalue_3 (/ _returnvalue 2.0))
  (bind _relativelocation (Variables|/Script/Engine.SceneComponent|GetRelativeLocation _colorframe))
  (bind (_x_2 _y_2) (Math|Vector2D|BreakVector2D _returnvalue_3))
  (bind _returnvalue_4 (Class|NeoKinectManager|SetUseFrame "Color" true))
  (bind _returnvalue_5 (Rendering|Material|CreateDynamicMaterialInstance (Variables|Default|GetColorFrame) 0 0 :!class /Script/Engine.PrimitiveComponent))
  (Rendering|Material|SetTextureParameterValue _returnvalue_5 "Texture" _returnvalue_4)
  (Camera|SetFieldOfView _camera (.X (Math|Vector2D|BreakVector2D _returnvalue)))
  (Class|CameraComponent|SetAspectRatio _camera (/ (Math|Conversions|ToFloat(Integer) _x) (Math|Conversions|ToFloat(Integer) _y)))
  (Transformation|SetRelativeScale3D (Variables|Default|GetColorFrame) (Math|Vector|MakeVector (* (Math|Trig|Tan(Degrees) _x_2) (.x _relativelocation) 0.01 2.0) (* (Math|Trig|Tan(Degrees) _y_2) (.x _relativelocation) 0.01 2.0) 0.0)))

(event EventBeginPlay
  (Class|NeoKinectManager|InitSensor)
  (Class|NeoKinectManager|SetUseJointsColorSpaceTransforms true)
  (bind _output_get (Variables|Default|SetFaces (Class|NeoKinectManager|GetFaces)))
  (for _array_element _output_get
    (bind _returnvalue (Game|SpawnActorfromClass "/Game/NeoKinectDemos/Blueprints/BP_Helmet.BP_Helmet_C" (Math|Transform|MakeTransform "0, 0, 0" "0, 0, 0" "1,1,1") "AlwaysSpawn" self _array_element 0))
    (Transformation|AttachComponentToComponent _returnvalue (Variables|Default|GetHelmets) "None" "SnapToTarget" "SnapToTarget" "SnapToTarget" true))
  (CallFunction|SetBackground))

(event EventEndPlay
  (params (EndPlayReason :type EEndPlayReason%20Enum :default "Destroyed"))
  (Class|NeoKinectManager|UninitSensor))

(event EventCallTriggerActor
  (Rendering|SetVisibility (Variables|Default|GetHowToEnterCamera) true false)
  (Input|EnableInput (Game|GetPlayerController 0)))

(event EventCallTriggerActorEndOverlap
  (Rendering|SetVisibility (Variables|Default|GetHowToEnterCamera) false false)
  (Input|DisableInput (Game|GetPlayerController 0))
  (CallFunction|ViewThroughKinect false))

(event Input|KeyboardEvents|E
  (params (Key :type Key%20Structure))
  (:Released
    (CallFunction|TogglePointOfView)))

(fn ConstructionScript)

(fn TogglePointOfView
  (CallFunction|ViewThroughKinect (not (Variables|Default|GetbIsViewingThroughKinect))))

(fn ViewThroughKinect
  (params (bViewThrough :type Boolean))
  (bind _returnvalue (Game|GetPlayerController 0))
  (bind _output_get (Variables|Default|SetbIsViewingThroughKinect bViewThrough))
  (if _output_get
    (Game|Player|SetViewTargetwithBlend _returnvalue self 0.5 "VTBlend_Linear" 0.0 false)
    (else
      (Game|Player|SetViewTargetwithBlend _returnvalue (Game|GetPlayerCharacter 0) 0.5 "VTBlend_Linear" 0.0 false))))